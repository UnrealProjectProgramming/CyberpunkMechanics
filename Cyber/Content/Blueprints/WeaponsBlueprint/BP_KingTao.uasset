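; BP_KingTao is a weapon Blueprint that picks a random nearby third-person character as its HomingTarget.
; Sphere overlap events maintain the OverlappedActors array, which Tick samples every frame while it is non-empty.
; The validity check and cast each roll their own random index, with an upper bound equal to the array length.
; Only actors that cast to TP_ThirdPersonCharacter become targets.
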(event OnComponentBeginOverlap(Sphere)
  (params (OverlappedComponent :type Primitive%20Component%20Object%20Reference) (OtherActor :type Actor%20Object%20Reference) (OtherComp :type Primitive%20Component%20Object%20Reference) (OtherBodyIndex :type Integer) (bFromSweep :type Boolean) (SweepResult :type Hit%20Result%20Structure%20%28by%20ref%29))
  (Utilities|Array|Add (Variables|Default|GetOverlappedActors) OtherActor))

(event OnComponentEndOverlap(Sphere)
  (params (OverlappedComponent :type Primitive%20Component%20Object%20Reference) (OtherActor :type Actor%20Object%20Reference) (OtherComp :type Primitive%20Component%20Object%20Reference) (OtherBodyIndex :type Integer))
  (Utilities|Array|RemoveItem (Variables|Default|GetOverlappedActors) OtherActor))

(event EventTick
  (params (DeltaSeconds :type Float%20%28single-precision%29))
  (bind _overlappedactors (Variables|Default|GetOverlappedActors))
  (bind _returnvalue (Utilities|Array|Length _overlappedactors))
  (bind _returnvalue_2 (Math|Random|RandomIntegerinRange 0 _returnvalue))
  (bind _output (Utilities|Array|Get(acopy) _overlappedactors _returnvalue_2))
  (if (not (== (Utilities|Array|Length _overlappedactors) 0))
    (Utilities|IsValid _output
      (:Is%20Valid
        (bind _astp_third_person_character (Utilities|Casting|CastToTP_ThirdPersonCharacter _output)
          (:then
            (Variables|Default|SetHomingTarget _astp_third_person_character))
          (:CastFailed
            (Development|PrintString "Failed")))))))

(fn ConstructionScript)